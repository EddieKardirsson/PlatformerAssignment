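; Platformer player character Blueprint that handles respawning, HUD upkeep and pause menu control.
; On destruction it asks PlatformerAssignmentGameMode to respawn it and recreates the HUD if none exists; BeginPlay caches the active HUD.
; A FlipFlop opens and closes the pause menu, switching game pause, mapping context and mouse cursor.
; Directional input steps the menu's index with modulo and moves keyboard focus to that item.
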(event Input|EnhancedActionEvents|EnhancedInputActionIA_Sprint
  (params (ActionValue :type Boolean) (ElapsedSeconds :type Float%20%28double-precision%29) (TriggeredSeconds :type Float%20%28double-precision%29) (InputAction :type Input%20Action%20Object%20Reference :default "/Game/ThirdPerson/Input/Actions/IA_Sprint.IA_Sprint")))

(event EventBeginPlay
  (bind _foundwidgets (Widget|GetAllWidgetsOfClass "/Game/Game/Blueprints/UI/WBP_HUD.WBP_HUD_C" true))
  (for _array_element _foundwidgets
    (Variables|Default|SetActiveHUD _array_element)))

(event Collision|EventActorBeginOverlap
  (params (OtherActor :type Actor%20Object%20Reference)))

(event EventTick
  (params (DeltaSeconds :type Float%20%28single-precision%29)))

(event EventOpenPauseMenu
  (bind _returnvalue (Game|GetPlayerController 0))
  (Utilities|FlowControl|FlipFlop
    (:A
      (bind _returnvalue_2 (UserInterface|CreateWidget "/Game/Game/Blueprints/UI/WBP_PauseMenu.WBP_PauseMenu_C"))
      (UserInterface|Viewport|AddtoViewport _returnvalue_2 0)
      (Game|SetGamePaused true)
      (Class|PlatformerAssignmentCharacter|AddPauseMenuMappingContext)
      (Variables|/Script/Engine.PlayerController|SetbShowMouseCursor _returnvalue true))
    (:B
      (Widget|RemovefromParent _returnvalue_2)
      (Game|SetGamePaused false)
      (Class|PlatformerAssignmentCharacter|RemovePauseMenuMappingContext)
      (Variables|/Script/Engine.PlayerController|SetbShowMouseCursor _returnvalue false))))

(event EventNavigateMenu
  (params (Value :type Input%20Action%20Value%20Structure%20%28by%20ref%29))
  (Variables|Default|SetNavigationInputValue Value)
  (Utilities|IsValid (Variables|Default|GetPauseMenu)
    (:Is%20Valid
      _)
    (:Is%20Not%20Valid
      (bind _foundwidgets (Widget|GetAllWidgetsOfClass "/Game/Game/Blueprints/UI/WBP_PauseMenu.WBP_PauseMenu_C" true))
      (for _array_element _foundwidgets
        (Variables|Default|SetPauseMenu _array_element))))
  (if (> (.y (Variables|Default|GetNavigationInputValue)) 0.0)
    (Variables|/Game/Game/Blueprints/UI/WBP_PauseMenu.WBP_PauseMenu_C|SetMenuNavigationIndex (Variables|Default|GetPauseMenu) (Math|Integer|%(Integer) (+ (Variables|/Game/Game/Blueprints/UI/WBP_PauseMenu.WBP_PauseMenu_C|GetMenuNavigationIndex (Variables|Default|GetPauseMenu)) 1) (Utilities|Array|Length (Variables|/Game/Game/Blueprints/UI/WBP_PauseMenu.WBP_PauseMenu_C|GetMenuItems (Variables|Default|GetPauseMenu)))))
    (else
      (Variables|/Game/Game/Blueprints/UI/WBP_PauseMenu.WBP_PauseMenu_C|SetMenuNavigationIndex (Variables|Default|GetPauseMenu) (Math|Integer|%(Integer) (- (Variables|/Game/Game/Blueprints/UI/WBP_PauseMenu.WBP_PauseMenu_C|GetMenuNavigationIndex (Variables|Default|GetPauseMenu)) 1) (Utilities|Array|Length (Variables|/Game/Game/Blueprints/UI/WBP_PauseMenu.WBP_PauseMenu_C|GetMenuItems (Variables|Default|GetPauseMenu)))))))
  (for (_array_element_2 _array_index) (Variables|/Game/Game/Blueprints/UI/WBP_PauseMenu.WBP_PauseMenu_C|GetMenuItems (Variables|Default|GetPauseMenu))
    (if (== _array_index (Variables|/Game/Game/Blueprints/UI/WBP_PauseMenu.WBP_PauseMenu_C|GetMenuNavigationIndex (Variables|Default|GetPauseMenu)))
      (Default|UpdateButtonState (Variables|Default|GetPauseMenu))
      (Widget|SetKeyboardFocus (Variables|Default|GetPauseMenu))
      (Utilities|FlowControl|Delay 0.2))))

(event Game|Damage|EventAnyDamage
  (params (Damage :type Float%20%28single-precision%29) (DamageType :type Damage%20Type%20Object%20Reference) (InstigatedBy :type Controller%20Object%20Reference) (DamageCauser :type Actor%20Object%20Reference)))

(event EventDeactivateHUD
  (Viewport|RemoveAllWidgets))

(event EventAfterDestroyed)

(event EventDestroyed
  (bind _asplatformer_assignment_game_mode (Utilities|Casting|CastToPlatformerAssignmentGameMode (Game|GetGameMode)))
  (Class|PlatformerAssignmentGameMode|RespawnPlayer _asplatformer_assignment_game_mode self)
  (bind _foundwidgets (Widget|GetAllWidgetsOfClass "/Game/Game/Blueprints/UI/WBP_HUD.WBP_HUD_C" true))
  (if (Utilities|Array|IsEmpty _foundwidgets)
    (bind _returnvalue (UserInterface|CreateWidget "/Game/Game/Blueprints/UI/WBP_HUD.WBP_HUD_C"))
    (UserInterface|Viewport|AddtoViewport _returnvalue 0)))

(fn ConstructionScript)